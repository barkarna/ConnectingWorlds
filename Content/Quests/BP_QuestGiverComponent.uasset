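; Actor component that makes its owner a quest giver, offering the quest referenced by its QuestData data table row handle.
; InteractWith asks the player character's quest log component whether that quest is already active.
; If not, DisplayQust looks up the row and prints the quest name; otherwise it prints an already-on-quest message.
; Both paths return the owner's display name, and the quest is only displayed, never added to the log.
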(fn `DisplayQust`
  (bind (_questdata_datatable _questdata_rowname) (break `DataTableRowHandle` (`self.QuestData`)))
  (bind _returnvalue (`|GetDataTableRow` _questdata_datatable _questdata_rowname)
    (:`then`
      (`KismetSystemLibrary.PrintString` (`KismetTextLibrary.Conv_TextToString` (`.QuestName_9_9642E5604B81BE9638316481D094516E` (break `/Game/Quests/S_QuestDetails` _returnvalue)))))))

(fn `InteractWith`
  (returns (ObjectiveID :type String))
  (bind (_questdata_datatable _questdata_rowname) (break `DataTableRowHandle` (`self.QuestData`)))
  (bind _returnvalue (`KismetSystemLibrary.GetDisplayName` (`self.GetOwner`)))
  (bind _myplayercharacter (`/Game/Blueprints/BPFL_Common.GetMyPlayerCharacter`))
  (if (not (`/Game/Quests/BP_QuestLogComponent.QueryActiveQuest` (`/Game/ThirdPerson/Blueprints/BP_ThirdPersonCharacter.BP_QuestLogComponent` _myplayercharacter) _questdata_rowname))
    (`self.DisplayQust`)
    (return _returnvalue)
    (else
      (`KismetSystemLibrary.PrintString` "Already on Quest")
      (return _returnvalue))))